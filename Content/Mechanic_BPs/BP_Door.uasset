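; BP_Door is an interactable, optionally locked door that swings open on its hinge.
; Interact checks the lock and asks the caller through a message whether it holds a key, then either uses the key, unlocks and opens, or shows an empty-text notification on CryptCharacter.
; Opening drives the hinge rotation with a timeline and, via Interact, hides the player's tutorial.
; The door's own HasKey always returns false.
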(event Custom|OpenDoor
  (bind _alpha (Timeline|DoorAnim Play)
    (:Update
      (Transformation|SetRelativeRotation (Variables|Default|GetMenteshe) (Math|Rotator|Lerp(Rotator) "0, 0, 0" "0.000000,90.000000,0.000000" _alpha) false false))))

(event EventBeginPlay)

(event Collision|EventActorBeginOverlap
  (params (OtherActor :type Actor%20Object%20Reference)))

(event EventTick
  (params (DeltaSeconds :type Float%20%28single-precision%29)))

(event EventInteract
  (params (Caller :type Actor%20Object%20Reference))
  (if (Variables|Default|GetbIsLocked)
    (if (Variables|Default|GetbRequiresKey)
      (bind _returnvalue (Class|InteractInterface|HasKey(Message) Caller))
      (if _returnvalue
        (bind _ascrypt_character (Utilities|Casting|CastToCryptCharacter (Game|GetPlayerCharacter 0)))
        (Class|InteractInterface|UseKey _ascrypt_character)
        (Variables|Default|SetbIsLocked false)
        (CallFunction|OpenDoor)
        (bind _ascrypt_character_2 (Utilities|Casting|CastToCryptCharacter (Game|GetPlayerCharacter 0)))
        (Class|CryptCharacter|HideTutorial _ascrypt_character_2)
        (else
          (bind _ascrypt_character_3 (Utilities|Casting|CastToCryptCharacter (Game|GetPlayerCharacter 0)))
          (Class|CryptCharacter|ShowNotification _ascrypt_character_3)))
      (else
        (bind _ascrypt_character_4 (Utilities|Casting|CastToCryptCharacter (Game|GetPlayerCharacter 0)))
        (Class|CryptCharacter|ShowNotification _ascrypt_character_4)))
    (else
      (CallFunction|OpenDoor)
      (bind _ascrypt_character_5 (Utilities|Casting|CastToCryptCharacter (Game|GetPlayerCharacter 0)))
      (Class|CryptCharacter|HideTutorial _ascrypt_character_5))))

(fn ConstructionScript)

(fn HasKey
  (return false))